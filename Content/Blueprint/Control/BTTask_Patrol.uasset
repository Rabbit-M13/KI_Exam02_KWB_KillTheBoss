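; Behavior tree task that walks an AI pawn along the patrol path defined on its BCP_AIBehavior component.
; At each point it notifies the patrol point of arrival, waits that point's mapped time, then signals exit and advances.
; At path ends it either loops to the start or reverses, per PatrolPathOutcome.
; The task runs continuously, finishing only as failure on a missing component, empty path or failed move.
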(event `self.ReceiveExecuteAI`
  (params (OwnerController :type "AIController Object Reference") (ControlledPawn :type "Pawn Object Reference"))
  (bind _returnvalue (`Actor.GetComponentByClass` ControlledPawn "/Game/Blueprint/Control/BCP_AIBehavior.BCP_AIBehavior_C"))
  (bind _patrolpath (`/Game/Blueprint/Control/BCP_AIBehavior.PatrolPath` _returnvalue))
  (set `self.Controlled Pawn` ControlledPawn)
  (`/Engine/EditorBlueprintResources/StandardMacros.IsValid` _returnvalue
    (:`Is Valid`
      (set `self.Patrol Path Outcome` (`/Game/Blueprint/Control/BCP_AIBehavior.PatrolPathOutcome` _returnvalue))
      (if (> (`BlueprintMapLibrary.Map_Length` _patrolpath) 0)
        (set `self.Patrol Path` _patrolpath)
        (`self.MoveToPatrolPoint`)
        (else
          (`self.FinishExecute` false))))
    (:`Is Not Valid`
      (`self.FinishExecute` false))))

(event `MoveToPatrolPoint`
  (bind _patrol_path (`self.Patrol Path`))
  (bind _keys (`BlueprintMapLibrary.Map_Keys` (`self.Patrol Path`)))
  (`|AIMoveTo` (`self.Controlled Pawn`) (`Actor.K2_GetActorLocation` (`|GetArrayItem` _keys (`self.CurrentPatrolIndex`))) null
    (:`OnSuccess`
      (bind _keys_2 (`BlueprintMapLibrary.Map_Keys` _patrol_path))
      (bind _output (`|GetArrayItem` _keys_2 (`self.CurrentPatrolIndex`)))
      (set `self.CurrentPatrolPoint` _output)
      (`KismetSystemLibrary.K2_SetTimerDelegate` (delegate `OnEndWaiting`) (`KismetMathLibrary.FMax` (`BlueprintMapLibrary.Map_Find` _patrol_path _output) 0.1))
      (`/Game/Blueprint/BP_Object/BP_AIPatrolPathPoint.OnPatrollerEntered` (`self.CurrentPatrolPoint`) (cast `Character` (`self.Controlled Pawn`) :!pure true)))
    (:`OnFail`
      (`self.FinishExecute` false))))

(event `OnEndWaiting`
  (`/Game/Blueprint/BP_Object/BP_AIPatrolPathPoint.OnPatrollerExit` (`self.CurrentPatrolPoint`))
  (bind _output_get (set `self.CurrentPatrolIndex` (+ (`self.CurrentPatrolIndex`) (`self.PathDirection`))))
  (if (`self.IsValidMapIndex` _output_get)
    (`self.MoveToPatrolPoint`)
    (else
      (switch `/Game/Blueprint/Control/E_PatrolPathOutcome` (`self.Patrol Path Outcome`)
        (:`NewEnumerator0`
          (set `self.CurrentPatrolIndex` 0)
          (`self.MoveToPatrolPoint`))
        (:`NewEnumerator1`
          (set `self.PathDirection` (* (`self.PathDirection`) -1))
          (set `self.CurrentPatrolIndex` (+ (`self.CurrentPatrolIndex`) (`self.PathDirection`)))
          (`self.MoveToPatrolPoint`))))))

(fn `IsValidMapIndex`
  (params (IndexToTest :type Integer))
  (returns (ReturnValue :type Boolean))
  (bind _keys (`BlueprintMapLibrary.Map_Keys` (`self.Patrol Path`)))
  (return (`KismetArrayLibrary.Array_IsValidIndex` _keys IndexToTest)))