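; AI controller for default enemies that runs their behavior tree and feeds it what the enemy sees and hears.
; On possess it sets up the BB_EnemyDefault blackboard and starts BT_EnemyDefault.
; Perception updates pass through sight and hearing handlers that write blackboard keys.
; Sight sets or clears the player target, saving the last seen location when lost, while hearing records the stimulus location from any source.
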(event `self.ReceivePossess`
  (params (PossessedPawn :type "Pawn Object Reference"))
  (bind _blackboardcomponent (`self.UseBlackboard` "/Game/Blueprint/Control/BB_EnemyDefault.BB_EnemyDefault"))
  (set `self.BBComp` _blackboardcomponent)
  (`self.RunBehaviorTree` "/Game/Blueprint/Control/BT_EnemyDefault.BT_EnemyDefault"))

(event `self.ReceiveBeginPlay`)

(event `self.AIPerception.OnTargetPerceptionUpdated`
  (params (Actor :type "Actor Object Reference") (Stimulus :type "AIStimulus Structure"))
  (`self.HandleSightSense` Actor Stimulus)
  (`self.HandleSoundSense` Stimulus))

(fn `HandleSightSense`
  (params (Actor :type "Actor Object Reference") (Stimulus :type "AIStimulus Structure"))
  (bind (_stimulus_age _stimulus_expirationage _stimulus_strength _stimulus_stimuluslocation _stimulus_receiverlocation _stimulus_tag _stimulus_bsuccessfullysensed) (break `AIStimulus` (`local.Stimulus`)))
  (bind _returnvalue (`AIPerceptionSystem.GetSenseClassForStimulus` Stimulus))
  (if (== _returnvalue "/Script/AIModule.AISense_Sight")
    (if (== (`local.Actor`) (`GameplayStatics.GetPlayerCharacter` 0))
      (`BlackboardComponent.SetValueAsObject` (`self.Blackboard`) "PlayerCharacter" (`KismetMathLibrary.SelectObject` (`GameplayStatics.GetPlayerCharacter` 0) null _stimulus_bsuccessfullysensed))
      (if (not _stimulus_bsuccessfullysensed)
        (`BlackboardComponent.SetValueAsVector` (`self.Blackboard`) "LastSeenLocation" _stimulus_stimuluslocation))
      (else
        (return)))
    (else
      (return))))

(fn `HandleSoundSense`
  (params (Stimulus :type "AIStimulus Structure (by ref)"))
  (bind _returnvalue (`AIPerceptionSystem.GetSenseClassForStimulus` Stimulus))
  (if (== _returnvalue "/Script/AIModule.AISense_Hearing")
    (`BlackboardComponent.SetValueAsVector` (`self.Blackboard`) "LastHearedLocation" (`.StimulusLocation` (break `AIStimulus` (`local.Stimulus`))))))

(fn `UserConstructionScript`)