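; Anim notify state that locks an AI enemy's movement and actions for a span of its animation.
; On begin it casts the mesh owner to BP_DefaultEnemy_AIPerception, clears ActionPlayable, disables character movement and makes its AI controller ignore move input.
; On end it restores ActionPlayable, sets the movement mode back to Walking and re-enables move input.
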(fn `Received_NotifyBegin`
  (params (MeshComp :type "SkeletalMeshComponent Object Reference") (Animation :type "AnimSequenceBase Object Reference") (TotalDuration :type "Float (single-precision)") (EventReference :type "AnimNotifyEventReference Structure (by ref)"))
  (returns (ReturnValue :type Boolean))
  (bind _asbp_default_enemy_aiperception (cast `/Game/Blueprint/BP_Character/BP_DefaultEnemy_AIPerception` (`ActorComponent.GetOwner` MeshComp)))
  (set `/Game/Blueprint/BP_Character/BP_DefaultEnemy_AIPerception.bActionPlayable` false _asbp_default_enemy_aiperception)
  (`CharacterMovementComponent.DisableMovement` (`Character.CharacterMovement` _asbp_default_enemy_aiperception))
  (bind `_asai_컨트롤러` (cast `AIController` (`Pawn.GetController` _asbp_default_enemy_aiperception)))
  (`Controller.SetIgnoreMoveInput` `_asai_컨트롤러` true)
  (return true))

(fn `Received_NotifyEnd`
  (params (MeshComp :type "SkeletalMeshComponent Object Reference") (Animation :type "AnimSequenceBase Object Reference") (EventReference :type "AnimNotifyEventReference Structure (by ref)"))
  (returns (ReturnValue :type Boolean))
  (bind _asbp_default_enemy_aiperception (cast `/Game/Blueprint/BP_Character/BP_DefaultEnemy_AIPerception` (`ActorComponent.GetOwner` MeshComp)))
  (set `/Game/Blueprint/BP_Character/BP_DefaultEnemy_AIPerception.bActionPlayable` true _asbp_default_enemy_aiperception)
  (`CharacterMovementComponent.SetMovementMode` (`Character.CharacterMovement` _asbp_default_enemy_aiperception) "MOVE_Walking" 0)
  (bind `_asai_컨트롤러` (cast `AIController` (`Pawn.GetController` _asbp_default_enemy_aiperception)))
  (`Controller.SetIgnoreMoveInput` `_asai_컨트롤러` false)
  (return true))