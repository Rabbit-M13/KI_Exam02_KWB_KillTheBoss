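; Patrol path point actor that turns an arriving AI character to face the direction of the point's arrow.
; Patroller entry stores the character, opens a Tick gate, prints a debug message and fires a point-met dispatcher; exit closes the gate.
; While the gate is open, Tick smoothly interpolates the character's rotation toward the arrow's world rotation.
; A note marks the entry event as the place for child classes to play a montage.
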(event `self.ReceiveTick`
  (params (DeltaSeconds :type "Float (single-precision)"))
  (`/Engine/EditorBlueprintResources/StandardMacros.Gate` true :!label _label
    (:`Exit`
      (`self.K2_SetActorRotation` (`self.Character_0`) (`KismetMathLibrary.RInterpTo` (`self.K2_GetActorRotation` (`self.Character_0`)) (`SceneComponent.K2_GetComponentRotation` (`self.Arrow_0`)) DeltaSeconds 2.0) false))))

(event `OnPatrollerExit`
  (goto _label :!via `Close`))

(event `OnPatrollerEntered`
  (params (Character :type "Character Object Reference"))
  (set `self.Character_0` Character)
  (`|ExecutionSequence`
    (:`then_0`
      (goto _label :!via `Open`))
    (:`then_1`
      ; 상속 받아서 여기서 몽타주 실행하자
      (`KismetSystemLibrary.PrintString` "Hello")
      (`self.OnPointMet_0`))))

(fn `UserConstructionScript`)