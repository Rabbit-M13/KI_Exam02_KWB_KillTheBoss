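; BP_Pistol is the player's hitscan pistol, attached as a child actor of BP_Player and bound to its silencer, fire and reload dispatchers.
; Firing checks the magazine, plays the matching sound, then line-traces from the camera to damage hit Characters.
; Shots report "Gunshot" noise events, quieter and shorter-ranged when silenced, with muzzle flash only unsilenced.
; Reload refills the magazine from reserve ammo; debug traces, prints and a silencer toggle remain.
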(event `self.ReceiveBeginPlay`
  (set `self.CurrentMag` (`self.MaxMag`))
  (bind _asbp_player (cast `/Game/Blueprint/BP_Character/BP_Player` (`self.GetParentActor`)))
  (bind _output_get (set `self.ParentCharacter` _asbp_player))
  ; BP_Player Crouch랑 연결되어 있음 추후 정정
  (add `/Game/Blueprint/BP_Character/BP_Player.ToggleSilencer` _output_get (`|CreateDelegate` :!event `ToggleShowSilencer`))
  (add `/Game/Blueprint/BP_Character/BP_Player.OnFire` _output_get (`|CreateDelegate` :!event `Fire`))
  (add `/Game/Blueprint/BP_Character/BP_Player.OnReload` _output_get (`|CreateDelegate` :!event `Reload`)))

(event `ShowPistol`
  ; 총 장착시 보이게 세팅
  (`SceneComponent.SetVisibility` (`self.Pistol`) false false))

(event `ToggleShowSilencer`
  ; 사용할 이벤트
  (if (`/Game/Blueprint/BP_Character/BP_Player.bHasSilencer` (`self.ParentCharacter`))
    (set `self.bIsSilencerOn` true)
    (`SceneComponent.SetVisibility` (`self.Silencer`) true false)
    (else
      (set `self.bIsSilencerOn` false)
      (`SceneComponent.SetVisibility` (`self.Silencer`) false false))))

(event `SetSilencerVisibility:Debug`
  ; Debug 이벤트
  (if (`self.bIsSilencerOn`)
    (`SceneComponent.SetVisibility` (`self.Silencer`) true false)
    (set `self.bIsSilencerOn` false)
    (else
      (`SceneComponent.SetVisibility` (`self.Silencer`) false false)
      (set `self.bIsSilencerOn` true))))

(event `Fire`
  (bind _returnvalue (`self.K2_GetActorLocation` (`GameplayStatics.GetPlayerCameraManager` 0)))
  ; 지금은 Debug 이벤트 때문에 소리 반대로 남 추후 ShowSilencer에서 제대로 동작하게 할 예정
  (`self.CurrentMagCheck`)
  (if (`self.bIsMagEmpty`)
    (`AudioComponent.Play` (`self.GunSound_EmptyFire`) 0.0)
    (else
      (if (`self.bIsSilencerOn`)
        (`AudioComponent.Play` (`self.GunSound_WithSilencer`) 0.0)
        (`AISense_Hearing.ReportNoiseEvent` (`SceneComponent.K2_GetComponentLocation` (`self.Pistol`)) 0.2 (`self.ParentCharacter`) 1000.0 "Gunshot")
        (else
          (`AudioComponent.Play` (`self.GunSound_NoSilencer`) 0.0)
          (`ActorComponent.Activate` (`self.Muzzle_Fire`) false)
          (`AISense_Hearing.ReportNoiseEvent` (`SceneComponent.K2_GetComponentLocation` (`self.Pistol`)) 1.0 (`self.ParentCharacter`) 2000.0 "Gunshot")))
      (set `self.CurrentMag` (- (`self.CurrentMag`) 1))
      ; 라인 트레이스 가상의 총알 발사
      (bind _outhit (`KismetSystemLibrary.LineTraceSingleForObjects` :`Start` _returnvalue :`End` (+ _returnvalue (* (`self.GetActorForwardVector` (`GameplayStatics.GetPlayerCameraManager` 0)) (`self.ShootRange`))) :`ObjectTypes` (`|MakeArray` "ObjectTypeQuery3" "ObjectTypeQuery1" "ObjectTypeQuery2" "ObjectTypeQuery4" :!type "EObjectTypeQuery Enum") :`DrawDebugType` "ForDuration"))
      (bind (_bblockinghit _binitialoverlap _time _distance _location _impactpoint _normal _impactnormal _physmat _hitactor) (`GameplayStatics.BreakHitResult` _outhit))
      (bind `_as캐릭터` (cast `Character` _hitactor))
      ;; Debug : LineTrace
      (`GameplayStatics.ApplyDamage` `_as캐릭터` 12.0)
      (`KismetSystemLibrary.PrintString` (`KismetSystemLibrary.GetDisplayName` _hitactor)))))

(event `CurrentMagCheck`
  (if (> (`self.CurrentMag`) 0)
    (set `self.bIsMagEmpty` false)
    (else
      (set `self.bIsMagEmpty` true)
      (set `self.CurrentMag` 0)
      ; UI로 대체해야함
      (`KismetSystemLibrary.PrintString` "재장전 필요!!" true true (struct :`G` 1.0 :`B` 0.480678 :`A` 1.0)))))

(event `Reload`
  (`AudioComponent.Play` (`self.GunSound_Reload`) 0.0)
  (if (> (`self.TotalAmmo`) 0)
    (if (>= (`self.TotalAmmo`) (`self.MaxMag`))
      (set `self.TotalAmmo` (- (`self.TotalAmmo`) (- (`self.MaxMag`) (`self.CurrentMag`))) :!label _label)
      (set `self.CurrentMag` (+ (`self.CurrentMag`) (- (`self.MaxMag`) (`self.CurrentMag`))))
      (set `self.bIsMagEmpty` false)
      (elif (> (+ (`self.TotalAmmo`) (`self.CurrentMag`)) (`self.MaxMag`))
        (goto _label)
        (else
          (set `self.CurrentMag` (+ (`self.CurrentMag`) (`self.TotalAmmo`)))
          (set `self.TotalAmmo` 0)
          (set `self.bIsMagEmpty` false))))
    (else
      (set `self.bIsMagEmpty` true))))

(fn `UserConstructionScript`)