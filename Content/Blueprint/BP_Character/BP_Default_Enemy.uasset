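; Default AI enemy character with health, melee attack and alert states, ending in a ragdoll death that stops AIC_EnemyDefault's logic.
; Toggle events switch patrol, suspicion, aggressive patrol and combat, setting speed or montages and firing dispatchers.
; Attack range-checks the blackboard player; punches use timer-looped socket sphere traces, damaging each actor once, while GunAttack is empty.
; A config-map state machine (RequestState/ApplyState) also exists, uncalled here.
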(event `self.ReceiveBeginPlay`
  ; Initialize Enemy Setting
  (set `CharacterMovementComponent.MaxWalkSpeed` (`self.PatrolSpeed`) (`self.CharacterMovement`))
  (`self.SetHealth` (`self.MaxHealth`))
  (set `self.CurrentState` "NewEnumerator0")
  (`KismetSystemLibrary.K2_SetTimerDelegate` (`|CreateDelegate` :!event `Attack`) 0.2 true))

(event `self.ReceiveAnyDamage`
  (params (Damage :type "Float (single-precision)") (DamageType :type "DamageType Object Reference") (InstigatedBy :type "Controller Object Reference") (DamageCauser :type "Actor Object Reference"))
  (`self.SetHealth` (- (`self.CurrentHealth`) Damage))
  (`self.PlayAnimMontage` "/Game/Animation/AM/AM_Enemy/Josh/AM_Enemy_Hit_Hard.AM_Enemy_Hit_Hard")
  (if (<= (`self.CurrentHealth`) 0.0)
    (`self.OnDeath`)))

(event `OnDeath`
  (bind _mesh (`self.Mesh`))
  (`/Engine/EditorBlueprintResources/StandardMacros.DoOnce` false
    (:`Completed`
      (set `self.bIsDead` true)
      (set `self.bActionPlayable` false)
      (bind _asaic_enemy_default (cast `/Game/Blueprint/Control/AIC_EnemyDefault` (`self.GetController`)))
      (`Controller.StopMovement` _asaic_enemy_default)
      (`BrainComponent.StopLogic` (`AIController.BrainComponent` _asaic_enemy_default) "Dead")
      (bind _bbcomp (`/Game/Blueprint/Control/AIC_EnemyDefault.BBComp` _asaic_enemy_default))
      (if (`KismetSystemLibrary.IsValid` _bbcomp)
        (`BlackboardComponent.SetValueAsBool` _bbcomp (`self.Key Name Dead`) true)
        (`CharacterMovementComponent.DisableMovement` (`self.CharacterMovement`))
        (`PrimitiveComponent.SetCollisionEnabled` (`self.CapsuleComponent`) "NoCollision")
        (`PrimitiveComponent.SetCollisionProfileName` _mesh "Ragdoll" true)
        (`PrimitiveComponent.SetSimulatePhysics` _mesh true)
        (`self.SetLifeSpan` 10.0)))))

(event `self.ReceiveTick`
  (params (DeltaSeconds :type "Float (single-precision)"))
  ; Attack Debuging
)

(event `Attack`
  (if (`self.bActionPlayable`)
    (if (not (`self.bIsDead`))
      (bind _asaic_enemy_default (cast `/Game/Blueprint/Control/AIC_EnemyDefault` (`self.GetController`)))
      (`/Engine/EditorBlueprintResources/StandardMacros.IsValid` _asaic_enemy_default
        (:`Is Valid`
          (bind `_as캐릭터` (cast `Character` (`BlackboardComponent.GetValueAsObject` (`AIBlueprintHelperLibrary.GetBlackboard` _asaic_enemy_default) (`self.Key Name PlayerCharacter`))))
          (if (`KismetSystemLibrary.IsValid` `_as캐릭터`)
            (if (<= (`KismetMathLibrary.VSize` (- (`self.K2_GetActorLocation`) (`self.K2_GetActorLocation` `_as캐릭터`))) 105.0)
              (set `self.bActionPlayable` false)
              (if (`self.bIsHoldingGun`)
                (`self.GunAttack`)
                (`KismetSystemLibrary.Delay` (`self.AttackCoolTime`))
                (set `self.bActionPlayable` true)
                (else
                  (`self.FistAttack`)
                  (`KismetSystemLibrary.Delay` (`self.AttackCoolTime`))
                  (set `self.bActionPlayable` true))))))))))

(event `GunAttack`)

(event `FistAttack`
  (`|PlayMontage` (`self.Mesh`) "/Game/Animation/AM/AM_Enemy/Josh/AM_Enemy_Punch_Left.AM_Enemy_Punch_Left"))

(event `/Game/Blueprint/BP_Anim/BPI_Enemy_Punch_Traces.End Punch Trace`
  (bind _punchtraceloop (`self.PunchTraceLoop`))
  (if (`KismetSystemLibrary.K2_IsValidTimerHandle` _punchtraceloop)
    (`KismetSystemLibrary.K2_ClearAndInvalidateTimerHandle` _punchtraceloop)
    (`BlueprintSetLibrary.Set_Clear` (`self.Hit Actor This Attack`))))

(event `/Game/Blueprint/BP_Anim/BPI_Enemy_Punch_Traces.Start Punch Trace`
  (`BlueprintSetLibrary.Set_Clear` (`self.Hit Actor This Attack`))
  (bind _returnvalue (`KismetSystemLibrary.K2_SetTimerDelegate` (delegate `PunchTrace`) 0.1 true))
  (set `self.PunchTraceLoop` _returnvalue))

(event `PunchTrace`
  (bind _mesh (`self.Mesh`))
  (bind _returnvalue_location (`KismetMathLibrary.BreakTransform` (`SceneComponent.GetSocketTransform` _mesh "LHand_Punch_Socket" "RTS_World")))
  (bind _returnvalue_location_2 (`KismetMathLibrary.BreakTransform` (`SceneComponent.GetSocketTransform` _mesh "LArm_Punch_Socket" "RTS_World")))
  (bind (_outhit _returnvalue) (`KismetSystemLibrary.SphereTraceSingleForObjects` :`Start` _returnvalue_location_2 :`End` _returnvalue_location :`Radius` 10.0 :`ObjectTypes` (`|MakeArray` "ObjectTypeQuery3" :!type "EObjectTypeQuery Enum") :`DrawDebugType` "ForDuration" :`TraceColor` (struct :`R` 0.484087 :`B` 1.0 :`A` 1.0) :`TraceHitColor` (struct :`R` 1.0 :`G` 0.985425 :`A` 1.0) :`DrawTime` 0.1))
  (if _returnvalue
    (bind (_bblockinghit _binitialoverlap _time _distance _location _impactpoint _normal _impactnormal _physmat _hitactor) (`GameplayStatics.BreakHitResult` _outhit))
    (`/Engine/EditorBlueprintResources/StandardMacros.IsValid` _hitactor
      (:`Is Valid`
        (if (not (`BlueprintSetLibrary.Set_Contains` (`self.Hit Actor This Attack`) _hitactor))
          (bind _asbp_player (cast `/Game/Blueprint/BP_Character/BP_Player` _hitactor))
          (`GameplayStatics.ApplyDamage` _asbp_player 2.0)
          (`BlueprintSetLibrary.Set_AddItems` (`self.Hit Actor This Attack`) (`|MakeArray` _hitactor)))))))

(event `StatePatrolToggle`
  (if (not (`self.bIsStatePatrol`))
    (set `self.bIsStatePatrol` true)
    (set `self.CurrentState` "NewEnumerator0")
    (set `CharacterMovementComponent.MaxWalkSpeed` (`self.PatrolSpeed`) (`self.CharacterMovement`))
    (`self.OnStatePatrol`)
    (`|ExecutionSequence`
      (:`then_0`
        (set `self.bIsStateAggresivePatrol` false))
      (:`then_1`
        (set `self.bIsStateSuspicion` false))
      (:`then_2`
        (set `self.bIsStateCombat` false)))))

(event `InSuspicion`
  (if (`self.bIsStateSuspicion`)
    (`self.OnAnimSusFinished`)
    ; 코멘트
    (set `self.bIsStateSuspicion` true)
    (else
      (set `self.bIsStateSuspicion` true)
      (set `self.CurrentState` "NewEnumerator1")
      (`|PlayMontage` (`self.Mesh`) "/Game/Animation/AM/AM_Enemy/Josh/AM_Enemy_Suspicion.AM_Enemy_Suspicion"
        (:`then`
          (`|ExecutionSequence`
            (:`then_0`
              (set `self.bIsStateAggresivePatrol` false))
            (:`then_1`
              (set `self.bIsStatePatrol` false))
            (:`then_2`
              (set `self.bIsStateCombat` false))
            (:`then_3`
              (set `self.bIsStateSuspicion` true))))
        (:`OnCompleted`
          (`self.OnAnimSusFinished` :!label _label)
          (bind _asaic_enemy_default (cast `/Game/Blueprint/Control/AIC_EnemyDefault` (`AIBlueprintHelperLibrary.GetAIController` self)))
          (`/Game/Blueprint/Control/AIC_EnemyDefault.OnSuspicionFinished` _asaic_enemy_default))
        (:`OnBlendOut`
          (goto _label))
        (:`OnInterrupted`
          (goto _label))))))

(event `StateAggresivePatrolToggle`
  (if (not (`self.bIsStateAggresivePatrol`))
    (set `self.bIsStateAggresivePatrol` true)
    (set `self.CurrentState` "NewEnumerator2")
    (set `CharacterMovementComponent.MaxWalkSpeed` (`self.AggPatrolSpeed`) (`self.CharacterMovement`))
    (`self.OnStateAggPatrol`)
    (`|ExecutionSequence`
      (:`then_0`
        (set `self.bIsStateSuspicion` false))
      (:`then_1`
        (set `self.bIsStatePatrol` false))
      (:`then_2`
        (set `self.bIsStateCombat` false)))))

(event `StateCombatToggle`
  (if (not (`self.bIsStateCombat`))
    (set `self.bIsStateCombat` true)
    (set `self.CurrentState` "NewEnumerator3")
    (set `CharacterMovementComponent.MaxWalkSpeed` (`self.CombatSpeed`) (`self.CharacterMovement`))
    (`self.OnStateCombat`)
    (`|ExecutionSequence`
      (:`then_0`
        (set `self.bIsStateSuspicion` false))
      (:`then_1`
        (set `self.bIsStatePatrol` false))
      (:`then_2`
        (set `self.bIsStateAggresivePatrol` false)))))

(event `OnLostTarget`
  (`|PlayMontage` (`self.Mesh`) "/Game/Animation/AM/AM_Enemy/Josh/AM_Enemy_Target_Lost.AM_Enemy_Target_Lost"
    (:`OnCompleted`
      (`self.OnAnimLostTargetFinished`))))

(fn `ApplyState`
  (params (NewState :type "/Game/Blueprint/BP_Character/ENUM_EnemyState Enum" :default "NewEnumerator0"))
  (bind _charactermovement (`self.CharacterMovement`))
  (bind (_currentconfig_movespeed _currentconfig_sightradius _currentconfig_losesightdelay _currentconfig_meleerange _currentconfig_shootingrange _currentconfig_brotatetomovement _currentconfig_entermontage) (break `/Game/Blueprint/BP_Character/ST_EnemyStateConfig` (`self.CurrentConfig`)))
  (bind (_value _returnvalue) (`BlueprintMapLibrary.Map_Find` (`self.StateConfigMap`) NewState))
  (if (`self.bIsTransitioning`)
    (`KismetSystemLibrary.PrintString` "Already transitioning" true true (struct :`R` 1.0 :`G` 0.007073 :`A` 1.0))
    (return)
    (elif (`|EnumInequality` NewState (`self.CurrentState`))
      (set `self.bIsTransitioning` true)
      ; <포인트>
      (`self.OnExit`)
      (if _returnvalue
        (set `self.CurrentConfig` _value)
        (set `self.CurrentState` NewState)
        (set `CharacterMovementComponent.MaxWalkSpeed` _currentconfig_movespeed _charactermovement)
        (bind _output_get (set `CharacterMovementComponent.bOrientRotationToMovement` _currentconfig_brotatetomovement _charactermovement))
        (set `CharacterMovementComponent.bUseControllerDesiredRotation` (not _output_get) _charactermovement)
        (`/Engine/EditorBlueprintResources/StandardMacros.IsValid` _currentconfig_entermontage
          (:`Is Valid`
            (`self.PlayAnimMontage` _currentconfig_entermontage)
            (`self.OnEnter` NewState)
            ; 추후 NotifyState로 변경 예정
            (set `self.bIsTransitioning` false)
            (return))
          (:`Is Not Valid`
            (return)))
        (else
          (`KismetSystemLibrary.PrintString` (`KismetStringLibrary.BuildString_Name` "Missing config for" "" (`|GetEnumeratorName` NewState)) true true (struct :`R` 1.0 :`G` 0.012732 :`A` 1.0))
          (set `self.bIsTransitioning` false)
          (return)))
      (else
        (set `self.bIsTransitioning` false)
        (return)))))

(fn `GetPatrolpointLocation`
  (returns (OutLocaton :type "Vector Structure"))
  (return (0.0 0.0 0.0)))

(fn `OnEnter`
  (params (NewState :type "/Game/Blueprint/BP_Character/ENUM_EnemyState Enum" :default "NewEnumerator0"))
  (bind _charactermovement (`self.CharacterMovement`))
  (bind (_currentconfig_movespeed _currentconfig_sightradius _currentconfig_losesightdelay _currentconfig_meleerange _currentconfig_shootingrange _currentconfig_brotatetomovement) (break `/Game/Blueprint/BP_Character/ST_EnemyStateConfig` (`self.CurrentConfig`)))
  (bind (_currentconfig_movespeed_2 _currentconfig_sightradius_2 _currentconfig_losesightdelay_2 _currentconfig_meleerange_2 _currentconfig_shootingrange_2 _currentconfig_brotatetomovement_2 _currentconfig_entermontage) (break `/Game/Blueprint/BP_Character/ST_EnemyStateConfig` (`self.CurrentConfig`)))
  (bind _output_get (set `CharacterMovementComponent.bOrientRotationToMovement` _currentconfig_brotatetomovement _charactermovement))
  (set `CharacterMovementComponent.bUseControllerDesiredRotation` (not _output_get) _charactermovement)
  (if (`KismetSystemLibrary.IsValid` _currentconfig_entermontage)
    (`self.PlayAnimMontage` _currentconfig_entermontage)
    (return)
    (else
      (return))))

(fn `OnExit`
  (bind (_currentconfig_movespeed _currentconfig_sightradius _currentconfig_losesightdelay _currentconfig_meleerange _currentconfig_shootingrange _currentconfig_brotatetomovement _currentconfig_entermontage) (break `/Game/Blueprint/BP_Character/ST_EnemyStateConfig` (`self.CurrentConfig`)))
  (if (`KismetSystemLibrary.IsValid` _currentconfig_entermontage)
    (`self.StopAnimMontage` _currentconfig_entermontage)
    (return)
    (else
      (return))))

(fn `RequestState`
  (params (NewState :type "/Game/Blueprint/BP_Character/ENUM_EnemyState Enum" :default "NewEnumerator0"))
  (if (`self.bIsTransitioning`)
    (`KismetSystemLibrary.PrintString` "Blocked: Transitioning")
    (return)
    (elif (and (`|EnumEquality` (`self.CurrentState`) "NewEnumerator5") (`|EnumInequality` NewState "NewEnumerator5"))
      (`KismetSystemLibrary.PrintString` "Blocked: DeadGuard" true true (struct :`G` 0.3575 :`B` 0.541667 :`A` 1.0))
      (return)
      (elif (`|EnumEquality` (`self.CurrentState`) NewState)
        (`KismetSystemLibrary.PrintString` "Blocked: SameState" true true (struct :`G` 0.051562 :`B` 0.078125 :`A` 1.0))
        (return)
        (else
          (`self.ApplyState` NewState))))))

(fn `SetHealth`
  (params (InHealth :type "Float (double-precision)"))
  (bind _output_get (set `self.CurrentHealth` InHealth))
  (`self.OnHealthChanged` _output_get))

(fn `UserConstructionScript`)