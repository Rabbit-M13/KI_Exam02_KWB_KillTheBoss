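; Debug sandbag that serves as a damage target, printing each hit's damage and playing an enemy hit animation.
; Health starts at max on BeginPlay and drops on AnyDamage, with SetHealth broadcasting OnHealthChanged after each update.
; Tick polls for zero health and once switches the mesh to simulated ragdoll physics.
; The actor stays in the world, as its DestroyActor node never runs.
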(event `self.ReceiveBeginPlay`
  (`self.SetHealth` (`self.MaxHealth`)))

(event `self.ReceiveAnyDamage`
  (params (Damage :type "Float (single-precision)") (DamageType :type "DamageType Object Reference") (InstigatedBy :type "Controller Object Reference") (DamageCauser :type "Actor Object Reference"))
  (`self.SetHealth` (- (`self.CurrentHealth`) Damage))
  (`KismetSystemLibrary.PrintString` (`KismetStringLibrary.BuildString_Double` "InDamage : " "" Damage) true true (struct :`R` 1.0 :`G` 0.059917 :`A` 1.0))
  (`SkeletalMeshComponent.PlayAnimation` (`self.Mesh`) "/Game/Animation/AM/AM_Enemy/AM_Enemy_Hit2.AM_Enemy_Hit2" false))

(event `self.ReceiveTick`
  (params (DeltaSeconds :type "Float (single-precision)"))
  (bind _mesh (`self.Mesh`))
  (if (<= (`self.CurrentHealth`) 0.0)
    (`/Game/OtherPackages/EditorBlueprintResources/StandardMacros.DoOnce` false
      (:`Completed`
        (`PrimitiveComponent.SetCollisionProfileName` _mesh "Ragdoll" true)
        (`PrimitiveComponent.SetSimulatePhysics` _mesh true)))))

(fn `SetHealth`
  (params (InHealth :type "Float (double-precision)"))
  (bind _output_get (set `self.CurrentHealth` InHealth))
  (`self.OnHealthChanged` _output_get))

(fn `UserConstructionScript`)