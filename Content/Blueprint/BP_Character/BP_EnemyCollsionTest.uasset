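; Enemy character Blueprint, apparently a test version, with a config-driven state machine that starts at patrol speed and full health.
; RequestState blocks changes during transitions, out of the dead state or into the current state, then calls ApplyState.
; ApplyState looks up StateConfigMap to set movement speed, rotation mode and enter montage.
; IsTransitioning stays set when a found config lacks a valid montage; the state toggle events are empty stubs.
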(event `self.ReceiveBeginPlay`
  ; Initialize Enemy Setting
  (set `CharacterMovementComponent.MaxWalkSpeed` (`self.PatrolSpeed`) (`self.CharacterMovement`))
  (set `self.CurrentHealth` (`self.MaxHealth`))
  (set `self.CurrentState` "NewEnumerator0"))

(event `StatePatrolToggle`)

(event `InSuspicion`)

(event `StateAggresivePatrolToggle`)

(event `StateCombatToggle`)

(fn `ApplyState`
  (params (NewState :type "/Game/Blueprint/BP_Character/ENUM_EnemyState Enum" :default "NewEnumerator0"))
  (bind _charactermovement (`self.CharacterMovement`))
  (bind (_currentconfig_movespeed _currentconfig_sightradius _currentconfig_losesightdelay _currentconfig_meleerange _currentconfig_shootingrange _currentconfig_brotatetomovement _currentconfig_entermontage) (break `/Game/Blueprint/BP_Character/ST_EnemyStateConfig` (`self.CurrentConfig`)))
  (bind (_value _returnvalue) (`BlueprintMapLibrary.Map_Find` (`self.StateConfigMap`) NewState))
  (if (`self.bIsTransitioning`)
    (`KismetSystemLibrary.PrintString` "Already transitioning" true true (struct :`R` 1.0 :`G` 0.007073 :`A` 1.0))
    (return)
    (elif (`|EnumInequality` NewState (`self.CurrentState`))
      (set `self.bIsTransitioning` true)
      ; <포인트>
      (`self.OnExit`)
      (if _returnvalue
        (set `self.CurrentConfig` _value)
        (set `self.CurrentState` NewState)
        (set `CharacterMovementComponent.MaxWalkSpeed` _currentconfig_movespeed _charactermovement)
        (bind _output_get (set `CharacterMovementComponent.bOrientRotationToMovement` _currentconfig_brotatetomovement _charactermovement))
        (set `CharacterMovementComponent.bUseControllerDesiredRotation` (not _output_get) _charactermovement)
        (`/Engine/EditorBlueprintResources/StandardMacros.IsValid` _currentconfig_entermontage
          (:`Is Valid`
            (`self.PlayAnimMontage` _currentconfig_entermontage)
            (`self.OnEnter` NewState)
            ; 추후 NotifyState로 변경 예정
            (set `self.bIsTransitioning` false)
            (return))
          (:`Is Not Valid`
            (return)))
        (else
          (`KismetSystemLibrary.PrintString` (`KismetStringLibrary.BuildString_Name` "Missing config for" "" (`|GetEnumeratorName` NewState)) true true (struct :`R` 1.0 :`G` 0.012732 :`A` 1.0))
          (set `self.bIsTransitioning` false)
          (return)))
      (else
        (set `self.bIsTransitioning` false)
        (return)))))

(fn `OnEnter`
  (params (NewState :type "/Game/Blueprint/BP_Character/ENUM_EnemyState Enum" :default "NewEnumerator0"))
  (bind _charactermovement (`self.CharacterMovement`))
  (bind (_currentconfig_movespeed _currentconfig_sightradius _currentconfig_losesightdelay _currentconfig_meleerange _currentconfig_shootingrange _currentconfig_brotatetomovement) (break `/Game/Blueprint/BP_Character/ST_EnemyStateConfig` (`self.CurrentConfig`)))
  (bind (_currentconfig_movespeed_2 _currentconfig_sightradius_2 _currentconfig_losesightdelay_2 _currentconfig_meleerange_2 _currentconfig_shootingrange_2 _currentconfig_brotatetomovement_2 _currentconfig_entermontage) (break `/Game/Blueprint/BP_Character/ST_EnemyStateConfig` (`self.CurrentConfig`)))
  (bind _output_get (set `CharacterMovementComponent.bOrientRotationToMovement` _currentconfig_brotatetomovement _charactermovement))
  (set `CharacterMovementComponent.bUseControllerDesiredRotation` (not _output_get) _charactermovement)
  (if (`KismetSystemLibrary.IsValid` _currentconfig_entermontage)
    (`self.PlayAnimMontage` _currentconfig_entermontage)
    (return)
    (else
      (return))))

(fn `OnExit`
  (bind (_currentconfig_movespeed _currentconfig_sightradius _currentconfig_losesightdelay _currentconfig_meleerange _currentconfig_shootingrange _currentconfig_brotatetomovement _currentconfig_entermontage) (break `/Game/Blueprint/BP_Character/ST_EnemyStateConfig` (`self.CurrentConfig`)))
  (if (`KismetSystemLibrary.IsValid` _currentconfig_entermontage)
    (`self.StopAnimMontage` _currentconfig_entermontage)
    (return)
    (else
      (return))))

(fn `RequestState`
  (params (NewState :type "/Game/Blueprint/BP_Character/ENUM_EnemyState Enum" :default "NewEnumerator0"))
  (if (`self.bIsTransitioning`)
    (`KismetSystemLibrary.PrintString` "Blocked: Transitioning")
    (return)
    (elif (and (`|EnumEquality` (`self.CurrentState`) "NewEnumerator5") (`|EnumInequality` NewState "NewEnumerator5"))
      (`KismetSystemLibrary.PrintString` "Blocked: DeadGuard" true true (struct :`G` 0.3575 :`B` 0.541667 :`A` 1.0))
      (return)
      (elif (`|EnumEquality` (`self.CurrentState`) NewState)
        (`KismetSystemLibrary.PrintString` "Blocked: SameState" true true (struct :`G` 0.051562 :`B` 0.078125 :`A` 1.0))
        (return)
        (else
          (`self.ApplyState` NewState))))))

(fn `UserConstructionScript`)