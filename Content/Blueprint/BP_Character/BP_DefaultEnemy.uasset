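; Default enemy character that walks a four-point patrol loop, takes damage and carries a guarded state machine.
; Overlapping a patrol point selects the next one and writes it to the Blackboard.
; RequestState blocks repeat, mid-transition and post-death changes, then ApplyState loads per-state movement and montage settings from StateConfigMap.
; Damage updates health, fires the health-changed dispatcher and plays a hit animation; several state events are empty stubs.
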(event `self.ReceiveActorBeginOverlap`
  (params (OtherActor :type "Actor Object Reference"))
  (if (== OtherActor (`self.PatrolPoints_0`))
    (set `self.CurrentPatrolPoint` (`self.PatrolPoints_1`))
    (`self.UpdatePatrolPointBB` :!label _label)
    (elif (== OtherActor (`self.PatrolPoints_1`))
      (set `self.CurrentPatrolPoint` (`self.PatrolPoints_2`))
      (goto _label)
      (elif (== OtherActor (`self.PatrolPoints_2`))
        (set `self.CurrentPatrolPoint` (`self.PatrolPoints_3`))
        (goto _label)
        (elif (== OtherActor (`self.PatrolPoints_3`))
          (set `self.CurrentPatrolPoint` (`self.PatrolPoints_0`))
          (goto _label))))))

(event `self.ReceiveBeginPlay`
  ; Initialize Enemy Setting
  (set `CharacterMovementComponent.MaxWalkSpeed` (`self.DebugSpeed`) (`self.CharacterMovement`))
  (`self.SetHealth` (`self.MaxHealth`))
  (set `self.CurrentState` "NewEnumerator0")
  (set `self.CurrentPatrolPoint` (`self.PatrolPoints_0`))
  (`self.UpdatePatrolPointBB`))

(event `self.ReceiveAnyDamage`
  (params (Damage :type "Float (single-precision)") (DamageType :type "DamageType Object Reference") (InstigatedBy :type "Controller Object Reference") (DamageCauser :type "Actor Object Reference"))
  (`self.SetHealth` (- (`self.CurrentHealth`) Damage))
  (`SkeletalMeshComponent.PlayAnimation` (`self.Mesh`) "/Game/Animation/AM/AM_Enemy/AM_Enemy_Hit_Hard.AM_Enemy_Hit_Hard" false)
  (`KismetSystemLibrary.PrintString` "Default Enemy Got Damaged" true true (struct :`R` 0.413929 :`B` 1.0 :`A` 1.0)))

(event `/Game/Blueprint/Control/BI_EnemyPatrolpoint.IncreasePatrolpointIndex`
  (bind _result (`/Engine/EditorBlueprintResources/StandardMacros.IncrementInt` (`self.PatrolpointIndex`))
    (:`  `
      (set `self.PatrolpointIndex` (mod _result (`KismetArrayLibrary.Array_Length` (`self.PatrolPoints`)))))))

(event `StatePatrolToggle`)

(event `InSuspicion`)

(event `StateAggresivePatrolToggle`)

(event `StateCombatToggle`)

(fn `ApplyState`
  (params (NewState :type "/Game/Blueprint/BP_Character/ENUM_EnemyState Enum" :default "NewEnumerator0"))
  (bind _charactermovement (`self.CharacterMovement`))
  (bind (_currentconfig_movespeed _currentconfig_sightradius _currentconfig_losesightdelay _currentconfig_meleerange _currentconfig_shootingrange _currentconfig_brotatetomovement _currentconfig_entermontage) (break `/Game/Blueprint/BP_Character/ST_EnemyStateConfig` (`self.CurrentConfig`)))
  (bind (_value _returnvalue) (`BlueprintMapLibrary.Map_Find` (`self.StateConfigMap`) NewState))
  (if (`self.bIsTransitioning`)
    (`KismetSystemLibrary.PrintString` "Already transitioning" true true (struct :`R` 1.0 :`G` 0.007073 :`A` 1.0))
    (return)
    (elif (`|EnumInequality` NewState (`self.CurrentState`))
      (set `self.bIsTransitioning` true)
      ; <포인트>
      (`self.OnExit`)
      (if _returnvalue
        (set `self.CurrentConfig` _value)
        (set `self.CurrentState` NewState)
        (set `CharacterMovementComponent.MaxWalkSpeed` _currentconfig_movespeed _charactermovement)
        (bind _output_get (set `CharacterMovementComponent.bOrientRotationToMovement` _currentconfig_brotatetomovement _charactermovement))
        (set `CharacterMovementComponent.bUseControllerDesiredRotation` (not _output_get) _charactermovement)
        (`/Engine/EditorBlueprintResources/StandardMacros.IsValid` _currentconfig_entermontage
          (:`Is Valid`
            (`self.PlayAnimMontage` _currentconfig_entermontage)
            (`self.OnEnter` NewState)
            ; 추후 NotifyState로 변경 예정
            (set `self.bIsTransitioning` false)
            (return))
          (:`Is Not Valid`
            (return)))
        (else
          (`KismetSystemLibrary.PrintString` (`KismetStringLibrary.BuildString_Name` "Missing config for" "" (`|GetEnumeratorName` NewState)) true true (struct :`R` 1.0 :`G` 0.012732 :`A` 1.0))
          (set `self.bIsTransitioning` false)
          (return)))
      (else
        (set `self.bIsTransitioning` false)
        (return)))))

(fn `GetPatrolpointLocation`
  (returns (OutLocaton :type "Vector Structure"))
  (return (0.0 0.0 0.0)))

(fn `OnEnter`
  (params (NewState :type "/Game/Blueprint/BP_Character/ENUM_EnemyState Enum" :default "NewEnumerator0"))
  (bind _charactermovement (`self.CharacterMovement`))
  (bind (_currentconfig_movespeed _currentconfig_sightradius _currentconfig_losesightdelay _currentconfig_meleerange _currentconfig_shootingrange _currentconfig_brotatetomovement) (break `/Game/Blueprint/BP_Character/ST_EnemyStateConfig` (`self.CurrentConfig`)))
  (bind (_currentconfig_movespeed_2 _currentconfig_sightradius_2 _currentconfig_losesightdelay_2 _currentconfig_meleerange_2 _currentconfig_shootingrange_2 _currentconfig_brotatetomovement_2 _currentconfig_entermontage) (break `/Game/Blueprint/BP_Character/ST_EnemyStateConfig` (`self.CurrentConfig`)))
  (bind _output_get (set `CharacterMovementComponent.bOrientRotationToMovement` _currentconfig_brotatetomovement _charactermovement))
  (set `CharacterMovementComponent.bUseControllerDesiredRotation` (not _output_get) _charactermovement)
  (if (`KismetSystemLibrary.IsValid` _currentconfig_entermontage)
    (`self.PlayAnimMontage` _currentconfig_entermontage)
    (return)
    (else
      (return))))

(fn `OnExit`
  (bind (_currentconfig_movespeed _currentconfig_sightradius _currentconfig_losesightdelay _currentconfig_meleerange _currentconfig_shootingrange _currentconfig_brotatetomovement _currentconfig_entermontage) (break `/Game/Blueprint/BP_Character/ST_EnemyStateConfig` (`self.CurrentConfig`)))
  (if (`KismetSystemLibrary.IsValid` _currentconfig_entermontage)
    (`self.StopAnimMontage` _currentconfig_entermontage)
    (return)
    (else
      (return))))

(fn `RequestState`
  (params (NewState :type "/Game/Blueprint/BP_Character/ENUM_EnemyState Enum" :default "NewEnumerator0"))
  (if (`self.bIsTransitioning`)
    (`KismetSystemLibrary.PrintString` "Blocked: Transitioning")
    (return)
    (elif (and (`|EnumEquality` (`self.CurrentState`) "NewEnumerator5") (`|EnumInequality` NewState "NewEnumerator5"))
      (`KismetSystemLibrary.PrintString` "Blocked: DeadGuard" true true (struct :`G` 0.3575 :`B` 0.541667 :`A` 1.0))
      (return)
      (elif (`|EnumEquality` (`self.CurrentState`) NewState)
        (`KismetSystemLibrary.PrintString` "Blocked: SameState" true true (struct :`G` 0.051562 :`B` 0.078125 :`A` 1.0))
        (return)
        (else
          (`self.ApplyState` NewState))))))

(fn `SetHealth`
  (params (InHealth :type "Float (double-precision)"))
  (bind _output_get (set `self.CurrentHealth` InHealth))
  (`self.OnHealthChanged` _output_get))

(fn `UserConstructionScript`)